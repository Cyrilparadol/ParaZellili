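; Plume is a collectible pickup that destroys itself when a BP_ThirdPersonCharacter overlaps it.
; Its Destroyed event spawns a pickup effect actor at the Sphere's location, then adds one to the score on BP_TopDownGameMode and calls CountFoodRemaining.
; Because the reward logic runs on Destroyed rather than on overlap, any destruction of the actor triggers the effect, and the score update whenever the game mode cast succeeds.
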(event EventDestroyed
  ;[1 1 1] Si destruction alors, spawn Vfx Explosion
  (Game|SpawnActorfromClass "/Game/StarterContent/Blueprints/Blueprint_Effect_Pickup.Blueprint_Effect_Pickup_C" (Math|Conversions|ToTransform(Vector) (Transformation|GetWorldLocation (Variables|Default|GetSphere))) "Undefined" "MultiplyWithRoot" 0 0)
  ;[1 1 1] Faire apparaître le score
  (bind _asbp_top_down_game_mode (Utilities|Casting|CastToBP_TopDownGameMode (Game|GetGameMode)))
  (Variables|/Game/TopDown/Blueprints/BP_TopDownGameMode.BP_TopDownGameMode_C|SetSCore _asbp_top_down_game_mode (+ (Variables|/Game/TopDown/Blueprints/BP_TopDownGameMode.BP_TopDownGameMode_C|GetSCore _asbp_top_down_game_mode) 1)) ; Défini le score
  (Default|CountFoodRemaining _asbp_top_down_game_mode))

(event Collision|EventActorBeginOverlap
  (params (OtherActor :type Actor%20Object%20Reference))
  (Utilities|Casting|CastToBP_ThirdPersonCharacter OtherActor)
  (Actor|DestroyActor))

(fn ConstructionScript)