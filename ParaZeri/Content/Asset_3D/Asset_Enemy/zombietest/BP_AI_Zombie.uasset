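; BP_AI_Zombie is an enemy zombie that chases the player and dies when its health runs out.
; Every Tick it reissues a simple move order toward the first player's character.
; AnyDamage subtracts from Health and prints the remaining value on screen.
; At zero health it enables ragdoll physics on the mesh, then destroys the actor immediately with no delay.
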(event Game|Damage|EventAnyDamage
  (params (Damage :type Float%20%28single-precision%29) (DamageType :type Damage%20Type%20Object%20Reference) (InstigatedBy :type Controller%20Object%20Reference) (DamageCauser :type Actor%20Object%20Reference))
  (bind _mesh (Variables|Character|GetMesh))
  ;[1 1 1] Take Damage, Ragdoll, Disparition
  (if (> (Variables|Default|GetHealth) 0.0)
    (Variables|Default|SetHealth (- (Variables|Default|GetHealth) Damage))
    (Development|PrintString (Utilities|String|ToString(Float) (Variables|Default|GetHealth)) true true "(R=1.000000,G=0.862090,B=0.241862,A=1.000000)")
    (if (<= (Variables|Default|GetHealth) 0.0)
      (Physics|SetSimulatePhysics _mesh true)
      (Class|SkeletalMeshComponent|SetPhysicsBlendWeight _mesh 1.0)
      (Collision|SetCollisionEnabled _mesh "QueryAndPhysics")
      (Actor|DestroyActor))))

(event EventTick
  (params (DeltaSeconds :type Float%20%28single-precision%29))
  (AI|Navigation|SimpleMovetoActor (Pawn|GetController) (Game|GetPlayerCharacter 0)))

(fn ConstructionScript)